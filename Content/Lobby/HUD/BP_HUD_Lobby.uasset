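; BP_HUD_Lobby is the lobby HUD that shows the lobby screen widget when play begins.
; On BeginPlay it calls EventLobbyInit, which creates WBP_Lobby only if no valid instance is stored, then adds it to the viewport.
; It then switches the first player controller to UI-only input with that widget focused.
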(event Custom|EventLobbyInit
  (Variables|Default|GetWBPLobby
    (:then
      _)
    (:else
      (bind _returnvalue (UserInterface|CreateWidget "/Game/Lobby/HUD/UI/WBP_Lobby.WBP_Lobby_C"))
      (Variables|Default|SetWBPLobby _returnvalue)))
  (UserInterface|Viewport|AddtoViewport (Variables|Default|GetWBPLobby) 0))

(event EventBeginPlay
  (Utilities|FlowControl|Sequence
    (:then_0
      (CallFunction|EventLobbyInit))
    (:then_1
      (Input|SetInputModeUIOnly (Game|GetPlayerController 0) (Variables|Default|GetWBPLobby) "DoNotLock" false))))

(event Collision|EventActorBeginOverlap
  (params (OtherActor :type Actor%20Object%20Reference)))

(event EventTick
  (params (DeltaSeconds :type Float%20%28single-precision%29)))

(fn ConstructionScript)