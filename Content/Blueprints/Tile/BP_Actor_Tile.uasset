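; Replicated spawn tile that one player at a time can claim as a unit spawn location.
; Game state phase updates make player controllers show spawn tiles during Planning for players without a unit, and hide them for Spells.
; Add and remove events toggle the claim and report the location to the player state.
; A RepNotify on the claiming player state tints the dynamic material as owned, taken or default.
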(event Custom|EventTilePhaseUpdate
  (params (Phase :type E_Phase%20Enum :default "NewEnumerator0"))
  (switch Utilities|FlowControl|Switch|SwitchonE_Phase Phase
    (:NewEnumerator1
      (bind _asbp_gs_gameplay (Utilities|Casting|CastToBP_GS_Gameplay (Game|GetGameState)))
      (for _array_element (Variables|/Script/Engine.GameStateBase|GetPlayerArray _asbp_gs_gameplay)
        (bind _asbp_ps_gameplay (Utilities|Casting|CastToBP_PS_Gameplay _array_element))
        (Variables|/Game/Gameplay/Player/BP_PS_Gameplay.BP_PS_Gameplay_C|GetUnit _asbp_ps_gameplay
          (:then)
          (:else
            (bind _asbp_pc_gameplay (Utilities|Casting|CastToBP_PC_Gameplay (Game|GetPlayerController _array_element)))
            (Default|EventPlayerControllerShowSpawnTiler _asbp_pc_gameplay true)))))
    (:NewEnumerator2
      (bind _asbp_gs_gameplay_2 (Utilities|Casting|CastToBP_GS_Gameplay (Game|GetGameState)))
      (for _array_element_2 (Variables|/Script/Engine.GameStateBase|GetPlayerArray _asbp_gs_gameplay_2)
        (bind _asbp_pc_gameplay_2 (Utilities|Casting|CastToBP_PC_Gameplay (Game|GetPlayerController _array_element_2)))
        (Default|EventPlayerControllerShowSpawnTiler _asbp_pc_gameplay_2 false)))))

(event Custom|EventTileAddPlayerstate
  (params (Playerstate :type Player%20State%20Object%20Reference))
  (Utilities|IsValid Playerstate
    (:Is%20Valid
      (bind _selected_player_state (Variables|Default|GetSelected%20Player%20State)
        (:then
          (if (== _selected_player_state Playerstate)
            (bind _asbp_ps_gameplay (Utilities|Casting|CastToBP_PS_Gameplay Playerstate))
            (Default|EventUpdateUnitSpawn _asbp_ps_gameplay false "0, 0, 0")
            (Variables|Default|SetSelected%20Player%20State 0)))
        (:else
          (Variables|Default|SetSelected%20Player%20State Playerstate)
          (bind _asbp_ps_gameplay_2 (Utilities|Casting|CastToBP_PS_Gameplay Playerstate))
          (Default|EventUpdateUnitSpawn _asbp_ps_gameplay_2 true (Transformation|GetActorLocation)))))))

(event Custom|EventTileRemovePlayerState
  (params (PlayerState :type Player%20State%20Object%20Reference))
  (Utilities|IsValid PlayerState
    (:Is%20Valid
      (bind _selected_player_state (Variables|Default|GetSelected%20Player%20State)
        (:then
          (if (== _selected_player_state PlayerState)
            (bind _asbp_ps_gameplay (Utilities|Casting|CastToBP_PS_Gameplay PlayerState))
            (Default|EventUpdateUnitSpawn _asbp_ps_gameplay false "0, 0, 0")
            (Variables|Default|SetSelected%20Player%20State 0)))
        (:else)))))

(event EventBeginPlay
  (bind _asbp_gs_gameplay (Utilities|Casting|CastToBP_GS_Gameplay (Game|GetGameState)))
  (EventDispatchers|BindEventtoOnPhaseUpdate _asbp_gs_gameplay (EventDispatchers|CreateEvent :!event Custom|EventTilePhaseUpdate))
  (Collision|SetCollisionResponsetoChannel (Variables|Default|GetCollision_Box) "ECC_GameTraceChannel3" "ECR_Block")
  (Collision|SetCollisionEnabled (Variables|Default|GetStaticMesh_Cube) "NoCollision")
  (Rendering|SetVisibility (Variables|Default|GetStaticMesh_Cube) false false)
  (Networking|SetReplicates true))

(event Collision|EventActorBeginOverlap
  (params (OtherActor :type Actor%20Object%20Reference)))

(event EventTick
  (params (DeltaSeconds :type Float%20%28single-precision%29)))

(fn ConstructionScript
  (bind _returnvalue (Rendering|Material|CreateDynamicMaterialInstance (Variables|Default|GetStaticMesh_Cube) 0 0 "None" :!class /Script/Engine.PrimitiveComponent))
  (Variables|Default|SetDMITile _returnvalue))

(fn OnRepSelectedPlayerState
  (bind _selected_player_state (Variables|Default|GetSelected%20Player%20State)
    (:then
      (if (== (Variables|/Script/Engine.Controller|GetPlayerState (Game|GetPlayerController 0)) _selected_player_state)
        (Rendering|Material|SetVectorParameterValue (Variables|Default|GetDMITile) "Color" (Variables|Default|GetOwnerColor) :!class /Script/Engine.MaterialInstanceDynamic)
        (else
          (Rendering|Material|SetVectorParameterValue (Variables|Default|GetDMITile) "Color" (Variables|Default|GetSelectedColor) :!class /Script/Engine.MaterialInstanceDynamic))))
    (:else
      (Rendering|Material|SetVectorParameterValue (Variables|Default|GetDMITile) "Color" (Variables|Default|GetDefaultColor) :!class /Script/Engine.MaterialInstanceDynamic))))