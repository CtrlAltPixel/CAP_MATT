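; BP_AC_AttributeSet is an attribute container component that builds and tracks an actor's attributes, each as its own component.
; EventAttributeInit adds every class in AttributeSet to the owner and stores it in the CurrentAttributes map, keyed by its display name.
; GetAttribute looks up entries by key.
; RemoveAttribute only removes the "None" key, and UpdateAttribute is an empty stub.
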(event Custom|EventAttributeInit
  (for _array_element (Variables|Default|GetAttributeSet)
    (CallFunction|AddAttribute _array_element)))

(event EventBeginPlay)

(event EventTick
  (params (DeltaSeconds :type Float%20%28single-precision%29)))

(fn GetAttribute
  (params (Key :type Name%20%28by%20ref%29))
  (bind _currentattributes (Variables|Default|GetCurrentAttributes))
  (bind (_value _returnvalue) (Utilities|Map|Find _currentattributes Key))
  (return _returnvalue _value))

(fn AddAttribute
  (params (InputPin :type Actor%20Component%20Class%20Reference))
  (bind _returnvalue (Game|AddComponentbyClass (Components|GetOwner) InputPin))
  (Utilities|Map|Add (Variables|Default|GetCurrentAttributes) (Utilities|String|StringToName (Utilities|GetDisplayName _returnvalue)) _returnvalue))

(fn RemoveAttribute
  (Utilities|Map|Remove (Variables|Default|GetCurrentAttributes) ""))

(fn UpdateAttribute
  (params (Key :type Name%20%28by%20ref%29)))