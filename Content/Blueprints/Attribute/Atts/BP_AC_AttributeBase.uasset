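; Base attribute Blueprint, apparently an actor component, that holds a stat as Base, Bonus, Multiplier, Current and Max values.
; CalculateAttribute sets Max to base plus bonus times the multiplier, as (Base + Bonus) * Multiplier, then resets Current to Max.
; RepNotifies on Current and Max fire OnAttributeUpdate with both values.
; ModifyAttribute only passes Value through, leaving its clamped subtraction from Current unconnected.
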(event EventBeginPlay)

(event EventTick
  (params (DeltaSeconds :type Float%20%28single-precision%29)))

(fn CalculateAttribute
  (bind _output_get (Variables|Default|SetMax (* (+ (Variables|Default|GetBase) (Variables|Default|GetBonus)) (Variables|Default|GetMultiplier))))
  (Variables|Default|SetCurrent _output_get))

(fn ModifyAttribute
  (params (Value :type Float%20%28double-precision%29))
  (bind _output_get (Variables|Default|SetValue Value)))

(fn OnRepCurrent
  (Default|CallOnAttributeUpdate (Variables|Default|GetCurrent) (Variables|Default|GetMax)))

(fn OnRepMax
  (Default|CallOnAttributeUpdate (Variables|Default|GetCurrent) (Variables|Default|GetMax)))