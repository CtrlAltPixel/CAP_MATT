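; Actor component that makes its owner detectable for interaction and gives it a ground decal highlight.
; On BeginPlay it sets the owner's interact capsule, fetched by message call, to block a custom trace channel.
; It then spawns a hidden decal at the owner's base, sized from its collision bounds plus padding, with a dynamic material instance.
; SetShowInteractDecal toggles the decal's visibility, while the component's own GetInteractCapsule is empty.
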(event Custom|EventDecalInit
  (bind _returnvalue (Components|GetOwner))
  (bind _boxextent (Collision|GetActorBounds _returnvalue true false))
  (Utilities|FlowControl|Sequence
    (:then_0
      (Variables|Default|GetDecal_Interact
        (:then)
        (:else
          (bind _returnvalue_2 (Class|GameplayStatics|SpawnDecalAttached "/Game/Blueprints/Interact/Material/MAT_Decal_Interact.MAT_Decal_Interact" (+ _boxextent 3e+01) (Variables|/Script/Engine.Actor|GetRootComponent _returnvalue) "None" (- (Transformation|GetActorLocation _returnvalue) (Math|Vector|MakeVector 0.0 0.0 (.Z (Math|Vector|BreakVector _boxextent)))) (Math|Conversions|RotationFromXVector (Transformation|GetActorUpVector _returnvalue)) "KeepWorldPosition" 0.0))
          (Variables|Default|SetDecal_Interact _returnvalue_2)
          (bind _returnvalue_3 (Rendering|Material|CreateDynamicMaterialInstance "/Game/Blueprints/Interact/Material/MAT_Decal_Interact.MAT_Decal_Interact" "None" "None" :!class /Script/Engine.KismetMaterialLibrary))
          (bind _output_get (Variables|Default|SetDecalMaterial _returnvalue_3))
          (Rendering|Components|Decal|SetDecalMaterial (Variables|Default|GetDecal_Interact) _output_get))))
    (:then_1
      (bind _decal_interact (Variables|Default|GetDecal_Interact)
        (:then
          (Rendering|SetVisibility _decal_interact false false))
        (:else)))))

(event EventBeginPlay
  (bind _capsulecollision (Class|BPIInteract|GetInteractCapsule(Message) (Components|GetOwner)))
  (Collision|SetCollisionResponsetoChannel _capsulecollision "ECC_GameTraceChannel1" "ECR_Block")
  (CallFunction|EventDecalInit))

(event EventTick
  (params (DeltaSeconds :type Float%20%28single-precision%29)))

(fn SetShowInteractDecal
  (params (Visibility :type Boolean))
  (bind _decal_interact (Variables|Default|GetDecal_Interact)
    (:then
      (Rendering|SetVisibility _decal_interact Visibility false))
    (:else)))

(fn GetInteractCapsule
  (return 0))