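; BP_AC_Target is a target component that highlights its owning actor's mesh with an overlay material while it is targeted.
; EventTargetInit creates and caches a dynamic instance of MAT_Overlay_Target.
; TargetStart applies that overlay to the mesh the owner returns through the GetTargetMesh message, and TargetEnd clears it.
; The component's own GetTargetMesh function is an empty stub.
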(event Custom|EventTargetInit
  (bind _returnvalue (Rendering|Material|CreateDynamicMaterialInstance "/Game/Blueprints/Target/Material/MAT_Overlay_Target.MAT_Overlay_Target" "None" "None" :!class /Script/Engine.KismetMaterialLibrary))
  (Variables|Default|SetMaterialOverlay _returnvalue))

(event EventBeginPlay)

(event EventTick
  (params (DeltaSeconds :type Float%20%28single-precision%29)))

(event EventTargetStart
  (bind _skeletalmesh (Class|BPITarget|GetTargetMesh(Message) (Components|GetOwner)))
  (Rendering|Material|SetOverlayMaterial _skeletalmesh (Variables|Default|GetMaterialOverlay) :!class /Script/Engine.MeshComponent))

(event EventTargetEnd
  (bind _skeletalmesh (Class|BPITarget|GetTargetMesh(Message) (Components|GetOwner)))
  (Rendering|Material|SetOverlayMaterial _skeletalmesh 0 :!class /Script/Engine.MeshComponent))

(fn GetTargetMesh
  (return 0))