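; Actor component that stores its owner's team (Blue, Neutral or Red) and marks it with a colored decal.
; BeginPlay spawns the decal attached at the bottom of the owner's bounds, sized to them and projected along its up axis, with a dynamic material instance.
; UpdateTeam stores the new team and recolors the decal to match.
; GetTeam returns the current team, while GetTeamCapsule is an empty stub.
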(event EventBeginPlay
  (bind _returnvalue (Components|GetOwner))
  (bind _boxextent (Collision|GetActorBounds _returnvalue true false))
  (Variables|Default|GetDecalTeam
    (:then)
    (:else
      (bind _returnvalue_2 (Class|GameplayStatics|SpawnDecalAttached "/Game/Blueprints/Team/Material/MAT_Decal_Team.MAT_Decal_Team" _boxextent (Variables|/Script/Engine.Actor|GetRootComponent _returnvalue) "None" (- (Transformation|GetActorLocation _returnvalue) (Math|Vector|MakeVector 0.0 0.0 (.Z (Math|Vector|BreakVector _boxextent)))) (Math|Conversions|RotationFromXVector (Transformation|GetActorUpVector _returnvalue)) "KeepWorldPosition" 0.0))
      (Variables|Default|SetDecalTeam _returnvalue_2)
      (bind _returnvalue_3 (Rendering|Material|CreateDynamicMaterialInstance "/Game/Blueprints/Team/Material/MAT_Decal_Team.MAT_Decal_Team" "None" "None" :!class /Script/Engine.KismetMaterialLibrary))
      (bind _output_get (Variables|Default|SetAsDecalMaterial _returnvalue_3))
      (Rendering|Components|Decal|SetDecalMaterial (Variables|Default|GetDecalTeam) _output_get))))

(event EventTick
  (params (DeltaSeconds :type Float%20%28single-precision%29)))

(event EventUpdateTeam
  (params (Team :type E_Team%20Enum :default "NewEnumerator0"))
  (bind _output_get (Variables|Default|SetTeam Team))
  (switch Utilities|FlowControl|Switch|SwitchonE_Team _output_get
    (:NewEnumerator1
      (Rendering|Components|Decal|SetDecalColor (Variables|Default|GetDecalTeam) (Variables|Default|GetBlueTeamColor)))
    (:NewEnumerator2
      (Rendering|Components|Decal|SetDecalColor (Variables|Default|GetDecalTeam) (Variables|Default|GetNeutralTeamColor)))
    (:NewEnumerator3
      (Rendering|Components|Decal|SetDecalColor (Variables|Default|GetDecalTeam) (Variables|Default|GetRedTeamColor)))))

(fn GetTeam
  (return (Variables|Default|GetTeam)))

(fn GetTeamCapsule
  (return 0))