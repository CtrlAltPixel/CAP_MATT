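; BP_AC_Weapon is a weapon component that shows its owner's main-hand and off-hand weapons from a WeaponData asset.
; On BeginPlay with valid data, or on a weapon change event, it updates both hands and notifies player 0's HUD.
; Each hand's BP_SM_Weapon is created through the owner at the right or left grip socket only if missing, then reused by swapping its mesh.
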(event Custom|EventWeaponChanged
  (params (WeaponData :type PDA%20Weapon%20Object%20Reference))
  (Variables|Default|SetWeaponData WeaponData)
  (CallFunction|InitWeapon (Variables|Default|GetWeaponData))
  (Class|BPIWeapon|UpdateWeaponUI(Message) (HUD|GetHUD (Game|GetPlayerController 0)) (Variables|Default|GetWeaponData)))

(event EventBeginPlay
  (bind _weapondata (Variables|Default|GetWeaponData)
    (:then
      (CallFunction|InitWeapon _weapondata)
      (Class|BPIWeapon|UpdateWeaponUI(Message) (HUD|GetHUD (Game|GetPlayerController 0)) (Variables|Default|GetWeaponData)))
    (:else)))

(event EventTick
  (params (DeltaSeconds :type Float%20%28single-precision%29)))

(fn GetWeaponData
  (return (Variables|Default|GetWeaponData)))

(fn InitWeapon
  (params (WeaponData :type PDA%20Weapon%20Object%20Reference))
  (CallFunction|UpdateMainHand WeaponData)
  (CallFunction|UpdateOffHand WeaponData)
  (return))

(fn UpdateMainHand
  (params (WeaponData :type PDA%20Weapon%20Object%20Reference))
  (Variables|Default|GetMainHandMesh
    (:then
      _)
    (:else
      (bind _weaponmeshcomponent (CallFunction|SpawnWeapon "HandGrip_R"))
      (Variables|Default|SetMainHandMesh _weaponmeshcomponent)))
  (Default|EventMeshUpdate (Variables|Default|GetMainHandMesh) (Variables|/Game/Blueprints/Weapon/Data/PDA_Weapon.PDA_Weapon_C|GetMainHandMesh WeaponData)))

(fn UpdateOffHand
  (params (WeaponData :type PDA%20Weapon%20Object%20Reference))
  (Variables|Default|GetOffHandMesh
    (:then
      _)
    (:else
      (bind _weaponmeshcomponent (CallFunction|SpawnWeapon "HandGrip_L"))
      (Variables|Default|SetOffHandMesh _weaponmeshcomponent)))
  (Default|EventMeshUpdate (Variables|Default|GetOffHandMesh) (Variables|/Game/Blueprints/Weapon/Data/PDA_Weapon.PDA_Weapon_C|GetOffHandMesh WeaponData)))

(fn SpawnWeapon
  (params (Socket%20Name :type Name))
  (bind _returnvalue (Game|AddComponentbyClass :self (Components|GetOwner) :Class "/Game/Blueprints/Weapon/BP_SM_Weapon.BP_SM_Weapon_C" :Socket%20Name Socket%20Name))
  (return _returnvalue))