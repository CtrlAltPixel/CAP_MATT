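; Gameplay player controller that routes Enhanced Input to the camera pawn and to cursor-based interaction.
; BeginPlay adds camera and interact mapping contexts, then camera actions forward move, rotate and zoom to the pawn.
; Primary interact traces under the cursor, messaging the hit actor and HUD, while secondary clears the selection.
; Target, tile, avatar and weapon graphs are mostly stubs, and their init events are not called here.
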(event EventBeginPlay
  ;[0.05098 0.05098 0.05098] Add Mapping Context
  (CallFunction|EventCameraInit)
  (CallFunction|EventInteractInit))

(event Custom|EventAvatarInit)

(event Custom|EventAvatarSpawn)

(event Custom|EventAvatarDeath)

(event Custom|EventCameraInit
  (bind _returnvalue (PlayerController|LocalPlayerSubsystems|GetEnhancedInputLocalPlayerSubsystem))
  (bind _asbp_pawn_camera (Utilities|Casting|CastToBP_Pawn_Camera (Pawn|GetControlledPawn)))
  (Variables|Default|SetBP_Pawn_Camera _asbp_pawn_camera)
  (Utilities|IsValid _returnvalue
    (:Is%20Valid
      (Input|AddMappingContext _returnvalue "/Game/Gameplay/Player/Input/IMC_Camera.IMC_Camera" 0 "(bIgnoreAllPressedKeysUntilRelease=True,bForceImmediately=False,bNotifyUserSettings=False)"))))

(event Input|EnhancedActionEvents|EnhancedInputActionIA_Camera_Move
  (params (ActionValue :type Vector%202D%20Structure) (ElapsedSeconds :type Float%20%28double-precision%29) (TriggeredSeconds :type Float%20%28double-precision%29) (InputAction :type Input%20Action%20Object%20Reference :default "/Game/Gameplay/Player/Input/Actions/Camera/IA_Camera_Move.IA_Camera_Move"))
  (:Started
    (bind _bp_pawn_camera (Variables|Default|GetBP_Pawn_Camera)
      (:then
        (Default|EventCameraMove _bp_pawn_camera (.x ActionValue) (.y ActionValue)))
      (:else))))

(event Input|EnhancedActionEvents|EnhancedInputActionIA_Camera_Rotate
  (params (ActionValue :type Float%20%28double-precision%29) (ElapsedSeconds :type Float%20%28double-precision%29) (TriggeredSeconds :type Float%20%28double-precision%29) (InputAction :type Input%20Action%20Object%20Reference :default "/Game/Gameplay/Player/Input/Actions/Camera/IA_Camera_Rotate.IA_Camera_Rotate"))
  (:Started
    (bind _bp_pawn_camera (Variables|Default|GetBP_Pawn_Camera)
      (:then
        (Default|EventCameraRotate _bp_pawn_camera ActionValue))
      (:else))))

(event Input|EnhancedActionEvents|EnhancedInputActionIA_Camera_Zoom
  (params (ActionValue :type Float%20%28double-precision%29) (ElapsedSeconds :type Float%20%28double-precision%29) (TriggeredSeconds :type Float%20%28double-precision%29) (InputAction :type Input%20Action%20Object%20Reference :default "/Game/Gameplay/Player/Input/Actions/Camera/IA_Camera_Zoom.IA_Camera_Zoom"))
  (:Started
    (bind _bp_pawn_camera (Variables|Default|GetBP_Pawn_Camera)
      (:then
        (Default|EventCameraZoom _bp_pawn_camera ActionValue))
      (:else))))

(event Custom|EventInteractInit
  (bind _returnvalue (PlayerController|LocalPlayerSubsystems|GetEnhancedInputLocalPlayerSubsystem))
  (Utilities|IsValid _returnvalue
    (:Is%20Valid
      (Input|AddMappingContext _returnvalue "/Game/Gameplay/Player/Input/IMC_Interact.IMC_Interact" 0 "(bIgnoreAllPressedKeysUntilRelease=True,bForceImmediately=False,bNotifyUserSettings=False)")
      (Variables|Default|SetCurrentClickTraceChannel "ECC_GameTraceChannel1")
      (Variables|Default|SetbEnableClickEvents true))))

(event Input|EnhancedActionEvents|EnhancedInputActionIA_Interact_Primary
  (params (ActionValue :type Boolean) (ElapsedSeconds :type Float%20%28double-precision%29) (TriggeredSeconds :type Float%20%28double-precision%29) (InputAction :type Input%20Action%20Object%20Reference :default "/Game/Gameplay/Player/Input/Actions/Interact/IA_Interact_Primary.IA_Interact_Primary"))
  (bind (_hit _hitactor) (CallFunction|ActorUnderCursorbyChannel "TraceTypeQuery3"))
  (:Started
    (bind _bp_actor_interact (Variables|Default|GetBP_Actor_Interact)
      (:then
        (Class|BPIInteract|EndInteract(Message) _bp_actor_interact))
      (:else
        _))
    (if _hit
      (bind _output_get (Variables|Default|SetBP_Actor_Interact _hitactor))
      (Class|BPIInteract|StartInteract(Message) _output_get)
      (Class|BPIInteract|UpdateInteractUI(Message) (HUD|GetHUD) _output_get)
      (else
        (Class|BPIInteract|UpdateInteractUI(Message) (HUD|GetHUD))))))

(event Input|EnhancedActionEvents|EnhancedInputActionIA_Interact_Secondary
  (params (ActionValue :type Boolean) (ElapsedSeconds :type Float%20%28double-precision%29) (TriggeredSeconds :type Float%20%28double-precision%29) (InputAction :type Input%20Action%20Object%20Reference :default "/Game/Gameplay/Player/Input/Actions/Interact/IA_Interact_Secondary.IA_Interact_Secondary"))
  (:Started
    (bind _bp_actor_interact (Variables|Default|GetBP_Actor_Interact)
      (:then
        (Class|BPIInteract|EndInteract(Message) _bp_actor_interact)
        (Class|BPIInteract|UpdateInteractUI(Message) (HUD|GetHUD)))
      (:else))))

(event Custom|EventTargetInit
  (bind _returnvalue (PlayerController|LocalPlayerSubsystems|GetEnhancedInputLocalPlayerSubsystem))
  (Utilities|IsValid _returnvalue
    (:Is%20Valid
      (Input|AddMappingContext _returnvalue "/Game/Gameplay/Player/Input/IMC_Target.IMC_Target" 0 "(bIgnoreAllPressedKeysUntilRelease=True,bForceImmediately=False,bNotifyUserSettings=False)"))))

(event Custom|EventTargetSpawn
  (bind _returnvalue (Game|SpawnActorfromClass "/Game/Blueprints/Target/BP_Actor_Target.BP_Actor_Target_C" (Math|Transform|MakeTransform "0, 0, 0" "0, 0, 0" "1.000000,1.000000,1.000000") "Undefined" "MultiplyWithRoot" 0 0 0))
  (Variables|Default|SetBP_Actor_Target _returnvalue))

(event Input|EnhancedActionEvents|EnhancedInputActionIA_Target_Primary
  (params (ActionValue :type Boolean) (ElapsedSeconds :type Float%20%28double-precision%29) (TriggeredSeconds :type Float%20%28double-precision%29) (InputAction :type Input%20Action%20Object%20Reference :default "/Game/Gameplay/Player/Input/Actions/Target/IA_Target_Primary.IA_Target_Primary")))

(event Input|EnhancedActionEvents|EnhancedInputActionIA_Target_Secondary
  (params (ActionValue :type Boolean) (ElapsedSeconds :type Float%20%28double-precision%29) (TriggeredSeconds :type Float%20%28double-precision%29) (InputAction :type Input%20Action%20Object%20Reference :default "/Game/Gameplay/Player/Input/Actions/Target/IA_Target_Secondary.IA_Target_Secondary")))

(event Custom|EventTilesInit
  (bind _returnvalue (PlayerController|LocalPlayerSubsystems|GetEnhancedInputLocalPlayerSubsystem))
  (Utilities|IsValid _returnvalue
    (:Is%20Valid
      (Input|AddMappingContext _returnvalue "/Game/Gameplay/Player/Input/IMC_Tile.IMC_Tile" 0 "(bIgnoreAllPressedKeysUntilRelease=True,bForceImmediately=False,bNotifyUserSettings=False)"))))

(event Input|EnhancedActionEvents|EnhancedInputActionIA_Tile_Primary
  (params (ActionValue :type Boolean) (ElapsedSeconds :type Float%20%28double-precision%29) (TriggeredSeconds :type Float%20%28double-precision%29) (InputAction :type Input%20Action%20Object%20Reference :default "/Game/Gameplay/Player/Input/Actions/Tile/IA_Tile_Primary.IA_Tile_Primary"))
  (bind (_hit _hitactor) (CallFunction|ActorUnderCursorbyChannel "TraceTypeQuery5"))
  (:Started
    (Variables|Default|GetBP_Actor_Tile
      (:then
        _)
      (:else
        _))
    (if _hit
      (Variables|Default|SetBP_Actor_Tile _hitactor))))

(event Input|EnhancedActionEvents|EnhancedInputActionIA_Tile_Secondary
  (params (ActionValue :type Boolean) (ElapsedSeconds :type Float%20%28double-precision%29) (TriggeredSeconds :type Float%20%28double-precision%29) (InputAction :type Input%20Action%20Object%20Reference :default "/Game/Gameplay/Player/Input/Actions/Tile/IA_Tile_Secondary.IA_Tile_Secondary"))
  (:Started
    (Variables|Default|GetBP_Actor_Tile
      (:then)
      (:else))))

(event Custom|EventWeaponInit)

(fn ConstructionScript)

(fn ActorUnderCursorbyChannel
  (params (TraceChannel :type ETraceTypeQuery%20Enum :default "TraceTypeQuery1"))
  (bind _hitresult (Game|Player|GetHitResultUnderCursorbyChannel TraceChannel true))
  (bind (_bblockinghit _binitialoverlap _time _distance _location _impactpoint _normal _impactnormal _physmat _hitactor) (Collision|BreakHitResult _hitresult))
  (return _bblockinghit _hitactor))