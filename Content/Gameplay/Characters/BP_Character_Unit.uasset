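; Base unit character Blueprint that supplies team, capsule and weapon mesh getters and reports its removal to the gameplay game mode.
; On BeginPlay it turns off decal reception on the mesh, and on Destroyed it passes itself to BP_GM_Gameplay's CallOnUnitDeath.
; The getters return a fixed team enum value, the capsule component for both interaction and team, and the character mesh as the weapon mesh.
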(event EventDestroyed
  (bind _asbp_gm_gameplay (Utilities|Casting|CastToBP_GM_Gameplay (Game|GetGameMode)))
  (Default|CallOnUnitDeath _asbp_gm_gameplay self))

(event EventBeginPlay
  (Rendering|SetReceivesDecals (Variables|Character|GetMesh) false))

(fn ConstructionScript)

(fn GetInteractCapsule
  (return (Variables|Collision|GetCapsuleComponent)))

(fn GetTeam
  (return "NewEnumerator0"))

(fn GetTeamCapsule
  (return (Variables|Collision|GetCapsuleComponent)))

(fn GetWeaponMesh
  (return (Variables|Character|GetMesh)))