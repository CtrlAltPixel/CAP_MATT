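; BP_HUD_Gameplay is the gameplay HUD Blueprint that creates and shows the main HUD, interact and weapon widgets.
; Each widget has its own init event, split across the event, interact and weapon graphs.
; Each event creates its widget only if the stored reference is invalid, caches it, then adds it to the viewport.
; Nothing runs on BeginPlay or Tick, and the init events are not called within this file.
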(event Custom|EventWBPHUDGameplayInit
  (Variables|Default|GetAsWBPHUDGameplay
    (:then
      _)
    (:else
      (bind _returnvalue (UserInterface|CreateWidget "/Game/Gameplay/HUD/UI/WBP_HUD.WBP_HUD_C"))
      (Variables|Default|SetAsWBPHUDGameplay _returnvalue)))
  (UserInterface|Viewport|AddtoViewport (Variables|Default|GetAsWBPHUDGameplay) 0))

(event EventBeginPlay)

(event Collision|EventActorBeginOverlap
  (params (OtherActor :type Actor%20Object%20Reference)))

(event EventTick
  (params (DeltaSeconds :type Float%20%28single-precision%29)))

(event Custom|EventWBPInteractInit
  (Variables|Default|GetAsWBPInteract
    (:then
      _)
    (:else
      (bind _returnvalue (UserInterface|CreateWidget "/Game/Blueprints/Interact/UI/WBP_Interact.WBP_Interact_C"))
      (Variables|Default|SetAsWBPInteract _returnvalue)))
  (UserInterface|Viewport|AddtoViewport (Variables|Default|GetAsWBPInteract) 0))

(event Custom|EventWBPWeaponInit
  (Variables|Default|GetAsWBPWeapon
    (:then
      _)
    (:else
      (bind _returnvalue (UserInterface|CreateWidget "/Game/Blueprints/Weapon/UI/WBP_Weapon.WBP_Weapon_C"))
      (Variables|Default|SetAsWBPWeapon _returnvalue)))
  (UserInterface|Viewport|AddtoViewport (Variables|Default|GetAsWBPWeapon) 0))

(fn ConstructionScript)