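; Game state that runs a phased, turn-based match, relaying match, turn, phase and action events to dispatchers.
; Phase start switches on the current phase: Spawn asks the game mode to spawn units at players' selected locations, then clears those selections.
; Ending an action starts another until the unit queue empties, then ends the phase.
; Queue filling is unfinished, and weapon locking, queue sorting and unit focus are empty stubs.
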(event EventBeginPlay)

(event EventTick
  (params (DeltaSeconds :type Float%20%28single-precision%29)))

(event Custom|EventMatchStart
  (Default|CallOnMatchStart))

(event Custom|EventMatchEnd
  (Default|CallOnMatchEnd))

(event Custom|EventMatchUpdate
  (Default|CallOnMatchUpdate))

(event Custom|EventTurnStart
  (Default|CallOnTurnStart))

(event Custom|EventTurnEnd
  (Default|CallOnTurnEnd))

(event Custom|EventTurnUpdate
  (Default|CallOnTurnUpdate))

(event Custom|EventPhaseStart
  (Default|CallOnPhaseStart)
  (switch Utilities|FlowControl|Switch|SwitchonE_Phase (Variables|Default|GetPhase)
    (:NewEnumerator1
      (CallFunction|UnlockWeapon))
    (:NewEnumerator2
      (CallFunction|LockWeapon)
      (CallFunction|CreateUnitQue))
    (:NewEnumerator3
      (CallFunction|CreateUnitQue))
    (:NewEnumerator4
      (CallFunction|CreateUnitQue))
    (:NewEnumerator5
      (CallFunction|CreateUnitQue))
    (:NewEnumerator8
      (CallFunction|CreateUnitQue))
    (:NewEnumerator6
      (CallFunction|CreateUnitQue))
    (:NewEnumerator7
      (Development|PrintString "switch to spawn")
      (CallFunction|SpawnUnits))))

(event Custom|EventPhaseEnd
  (Default|CallOnPhaseEnd))

(event Custom|EventPhaseUpdate
  (params (Phase :type E_Phase%20Enum :default "NewEnumerator0"))
  (bind _output_get (Variables|Default|SetPhase Phase))
  (Default|CallOnPhaseUpdate _output_get))

(event Custom|EventActionStart
  (Default|CallOnActionStart))

(event Custom|EventActionUpdate
  (Default|CallOnActionUpdate))

(event Custom|EventActionEnd
  (Default|CallOnActionEnd)
  (if (Utilities|Array|IsEmpty (Variables|Default|GetUnitQue))
    (CallFunction|EventPhaseEnd)
    (else
      (CallFunction|EventActionStart))))

(fn ConstructionScript)

(fn UnlockWeapon)

(fn LockWeapon)

(fn CreateUnitQue
  (bind _outactors (Actor|GetAllActorsOfClass "/Game/Gameplay/Characters/BP_Character_Unit.BP_Character_Unit_C"))
  (for _array_element _outactors
    (switch Utilities|FlowControl|Switch|SwitchonE_Phase (Variables|Default|GetPhase)))
  (return))

(fn SortUnitQue)

(fn SpawnUnits
  (for _array_element (Variables|Default|GetPlayerArray)
    (bind _asbp_ps_gameplay (Utilities|Casting|CastToBP_PS_Gameplay _array_element))
    (if (Variables|/Game/Gameplay/Player/BP_PS_Gameplay.BP_PS_Gameplay_C|GetbSpawnSelected? _asbp_ps_gameplay)
      (bind _asbp_gm_gameplay (Utilities|Casting|CastToBP_GM_Gameplay (Game|GetGameMode)))
      (Default|EventUnitSpawn _asbp_gm_gameplay (Variables|/Game/Gameplay/Player/BP_PS_Gameplay.BP_PS_Gameplay_C|GetSpawnLocation _asbp_ps_gameplay) 0 (Game|GetPlayerController _array_element))
      (Default|EventUpdateUnitSpawn _asbp_ps_gameplay false "0, 0, 0")))
  (Development|PrintString "Function spawn"))

(fn FocusUnit)