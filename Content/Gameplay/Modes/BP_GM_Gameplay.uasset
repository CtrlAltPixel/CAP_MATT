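; Gameplay game mode that spawns commandable units and tracks connected player controllers.
; A spawn event creates a unit linked to its commanding player controller, then has a new gameplay AI controller possess it.
; Login and logout maintain the controller list, and controller swaps touch the loadout message.
; It binds to unit deaths at BeginPlay, and the death handler's team switch has no actions yet.
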(event Custom|EventUnitSpawn
  (params (SpawnLocation :type Vector) (PlayerController :type Player%20Controller%20Object%20Reference))
  (bind _returnvalue (Game|SpawnActorfromClass "/Game/Gameplay/Characters/BP_Character_Unit.BP_Character_Unit_C" (Math|Transform|MakeTransform SpawnLocation "0, 0, 0" "1.000000,1.000000,1.000000") "Undefined" "MultiplyWithRoot" 0 PlayerController 0))
  (bind _returnvalue_2 (Game|SpawnActorfromClass "/Game/Gameplay/Characters/AI/BP_AIC_Gameplay.BP_AIC_Gameplay_C" (Math|Transform|MakeTransform "0, 0, 0" "0, 0, 0" "1.000000,1.000000,1.000000") "Undefined" "MultiplyWithRoot" 0 0))
  (Pawn|Possess _returnvalue_2 _returnvalue))

(event Custom|EventUnitDeath
  (params (Unit :type Character%20Object%20Reference))
  (bind _returnvalue (Actor|GetComponentbyClass Unit "/Game/Blueprints/Team/BP_AC_Team.BP_AC_Team_C"))
  (Utilities|IsValid _returnvalue
    (:Is%20Valid
      (switch Utilities|FlowControl|Switch|SwitchonE_Team (Variables|/Game/Blueprints/Team/BP_AC_Team.BP_AC_Team_C|GetTeam _returnvalue)))))

(event EventBeginPlay
  (EventDispatchers|BindEventtoOnUnitDeath (EventDispatchers|CreateEvent :!event Custom|EventUnitDeath)))

(event EventTick
  (params (DeltaSeconds :type Float%20%28single-precision%29)))

(event EventPostLogin
  (params (NewPlayer :type Player%20Controller%20Object%20Reference))
  (Utilities|Array|Add (Variables|Default|GetConnectedPlayerController) NewPlayer))

(event EventOnLogout
  (params (ExitingController :type Controller%20Object%20Reference))
  (bind _asbp_pc_gameplay (Utilities|Casting|CastToBP_PC_Gameplay ExitingController))
  (Utilities|Array|RemoveItem (Variables|Default|GetConnectedPlayerController) _asbp_pc_gameplay))

(event EventOnSwapPlayerControllers
  (params (OldPC :type Player%20Controller%20Object%20Reference) (NewPC :type Player%20Controller%20Object%20Reference))
  (Class|BPILobby|GetLoadout(Message) OldPC)
  (Class|BPILobby|SetLoadout(Message) NewPC false))

(fn ConstructionScript)